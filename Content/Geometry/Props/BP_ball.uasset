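; BP_ball is a ball prop that varies its look through randomization in the Construction Script.
; It gives the BalleLow mesh a random relative roll and pitch, while yaw stays effectively fixed because its random range has identical bounds.
; A random integer then selects one of three material instances for the mesh's first slot.
; The event graph holds only disabled placeholder events, so there is no runtime logic.
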(fn `UserConstructionScript`
  (bind _balle_low (`self.Balle_low`))
  (set `self.Selection` (`KismetMathLibrary.RandomIntegerInRange` 0 2))
  (set `self.New Rotation X (Roll)` (`KismetMathLibrary.RandomFloatInRange` -70.0 70.0))
  (set `self.New Rotation Y (Pitch)` (`KismetMathLibrary.RandomFloatInRange` -70.0 70.0))
  (set `self.New Rotation Z (Yaw)` (`KismetMathLibrary.RandomFloatInRange` -360.0 -360.0))
  (`SceneComponent.K2_SetRelativeRotation` (`self.Balle_low`) (`KismetMathLibrary.MakeRotator` (`self.New Rotation X (Roll)`) (`self.New Rotation Y (Pitch)`) (`self.New Rotation Z (Yaw)`)) false false)
  (switch `int` (`self.Selection`)
    (:`Default`
      (`PrimitiveComponent.SetMaterial` _balle_low 0 "/Game/Mesh/Props/BALL_ALBEDO_Mat_Inst.BALL_ALBEDO_Mat_Inst" :!label _label))
    (:`0`
      (goto _label))
    (:`1`
      (`PrimitiveComponent.SetMaterial` _balle_low 0 "/Game/Mesh/Props/BALL_ALBEDO_Mat_Inst1.BALL_ALBEDO_Mat_Inst1"))
    (:`2`
      (`PrimitiveComponent.SetMaterial` _balle_low 0 "/Game/Mesh/Props/BALL_ALBEDO_Mat_Inst2.BALL_ALBEDO_Mat_Inst2"))))