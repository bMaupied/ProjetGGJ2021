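; BP_Parasol is a parasol prop that randomizes its orientation, with no active gameplay logic.
; Its construction script rotates the ParasolBaseLow component twice: first with a slight random roll and random yaw, then with random yaw alone.
; The second call sets roll back to zero on the same component, so only the random yaw remains.
; The event graph holds only disabled default events.
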(fn `UserConstructionScript`
  (`SceneComponent.K2_SetRelativeRotation` (`self.Parasol_Base_low`) (`KismetMathLibrary.MakeRotator` (`KismetMathLibrary.RandomFloatInRange` -15.0 15.0) 0.0 (`KismetMathLibrary.RandomFloatInRange` 0.0 360.0)) false false)
  (`SceneComponent.K2_SetRelativeRotation` (`self.Parasol_Base_low`) (`KismetMathLibrary.MakeRotator` 0.0 0.0 (`KismetMathLibrary.RandomFloatInRange` 0.0 360.0)) false false))