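; BP_Canette is a prop made of several can meshes that varies its look by randomly showing or hiding them.
; The construction script applies unseeded random booleans to the visibility of overlapping groups of cans, so the layout can change on each reconstruction.
; Random integer switches sit between the groups, but their wired branches converge on the same next step.
; The event graph holds only disabled placeholder events.
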(fn `UserConstructionScript`
  (locals (NewLocalVar_0 :type Boolean :default false))
  (`SceneComponent.SetVisibility` (`self.Canette_low`) (`KismetMathLibrary.RandomBool`) false)
  (`SceneComponent.SetVisibility` (`self.Canette_low2`) (`KismetMathLibrary.RandomBool`) false)
  (`SceneComponent.SetVisibility` (`self.Canette_low5`) (`KismetMathLibrary.RandomBool`) false)
  (switch `int` (`KismetMathLibrary.RandomIntegerInRange` 0 2)
    (:`Default`
      _)
    (:`0`
      _))
  (`SceneComponent.SetVisibility` (`self.Canette_low3`) (`KismetMathLibrary.RandomBool`) false)
  (`SceneComponent.SetVisibility` (`self.Canette_low4`) (`KismetMathLibrary.RandomBool`) false)
  (`SceneComponent.SetVisibility` (`self.Canette_low1`) (`KismetMathLibrary.RandomBool`) false)
  (`SceneComponent.SetVisibility` (`self.Canette_low6`) (`KismetMathLibrary.RandomBool`) false)
  (`SceneComponent.SetVisibility` (`self.Canette_low9`) (`KismetMathLibrary.RandomBool`) false)
  (`SceneComponent.SetVisibility` (`self.Canette_low2`) (`KismetMathLibrary.RandomBool`) false)
  (switch `int` (`KismetMathLibrary.RandomIntegerInRange` 0 2)
    (:`Default`
      _)
    (:`0`
      _))
  (`SceneComponent.SetVisibility` (`self.Canette_low7`) (`KismetMathLibrary.RandomBool`) false)
  (`SceneComponent.SetVisibility` (`self.Canette_low8`) (`KismetMathLibrary.RandomBool`) false))