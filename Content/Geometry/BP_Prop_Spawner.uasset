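; BP_Prop_Spawner places one randomly chosen prop from its Props class list in the level.
; At BeginPlay it spawns that prop at the PreviewMesh world location with zero rotation and unit scale.
; A separate Sync function scans prop class-default mesh bounds, raising MaxSize to the largest max-bound component.
; Whenever MaxSize grows, PreviewMesh takes the mesh from BP_Prop's class defaults, not from the prop being measured.
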(event `self.ReceiveBeginPlay`
  (`|SpawnActorFromClass` (`KismetArrayLibrary.Array_Random` (`self.Props`)) (`KismetMathLibrary.MakeTransform` (`SceneComponent.K2_GetComponentLocation` (`self.PreviewMesh`))) "Undefined" "OverrideRootScale" null null))

(fn `Sync`
  (locals (`Max size` :type "Float (double-precision)"))
  (for _array_element (`self.Props`)
    (bind _returnvalue (`KismetMathLibrary.FMax` (.x (`.Max` (break `Box` (`StaticMesh.GetBoundingBox` (`.MeshComponent` (defaults `Object` _array_element)))))) (.y (`.Max` (break `Box` (`StaticMesh.GetBoundingBox` (`.MeshComponent` (defaults `Object` _array_element)))))) (.z (`.Max` (break `Box` (`StaticMesh.GetBoundingBox` (`.MeshComponent` (defaults `Object` _array_element))))))))
    (if (> _returnvalue (`local.Max size`))
      (set `local.Max size` _returnvalue)
      (`StaticMeshComponent.SetStaticMesh` (`self.PreviewMesh`) (`.MeshComponent` (defaults `/Game/Geometry/Spawnable/BP_Prop` "/Game/Geometry/Spawnable/BP_Prop.BP_Prop_C"))))))

(fn `UserConstructionScript`)